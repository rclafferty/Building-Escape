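; BP_OpenableDoor is a door actor that swings open and closed when its OpenDoor member fires open or close events.
; It stores its starting rotation and location, then plays or reverses the DoorSwing timeline, adding the timeline's yaw angle to that initial rotation.
; An event track on the timeline triggers the Doorlock sound at the door's starting location.
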(event OnOpen(OpenDoor)
  (bind _open_angle (Timeline|Door%20Swing Play)
    (:Update
      (Transformation|SetActorRotation (Math|Rotator|CombineRotators (Variables|Default|GetInitial%20Rotation) (Math|Rotator|MakeRotator 0.0 0.0 _open_angle))))
    (:Sound%20Timing
      (Audio|PlaySoundatLocation "/Game/Audio/door-lock.door-lock" (Variables|Default|GetInitial%20Location) "0, 0, 0" 1.0 1.0 0.0 0 0 0))))

(event OnClose(OpenDoor)
  (bind _open_angle (Timeline|Door%20Swing Reverse)
    (:Update
      (Transformation|SetActorRotation (Math|Rotator|CombineRotators (Variables|Default|GetInitial%20Rotation) (Math|Rotator|MakeRotator 0.0 0.0 _open_angle))))
    (:Sound%20Timing
      (Audio|PlaySoundatLocation "/Game/Audio/door-lock.door-lock" (Variables|Default|GetInitial%20Location) "0, 0, 0" 1.0 1.0 0.0 0 0 0))))

(event EventBeginPlay
  (Variables|Default|SetInitial%20Rotation (Transformation|GetActorRotation))
  (Variables|Default|SetInitial%20Location (Transformation|GetActorLocation)))

(fn ConstructionScript)